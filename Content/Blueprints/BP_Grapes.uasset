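; Pickable grapes actor that the first-person player collects through an Interact event.
; BeginPlay enables click events, destroys the actor if IsPicked is set, and otherwise applies a purple (red) or green (white) material from RedOrWhite.
; Interact calls DestroyActor first, then calls AddGrapes on BP_FirstPersonCharacter, sets IsPicked, and separately increments and prints the character's NumGrapes.
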(event EventBeginPlay
  (Variables|/Script/Engine.PlayerController|SetbEnableClickEvents (Game|GetPlayerController 0) true)
  (if (Variables|Default|GetisPicked)
    (Actor|DestroyActor)
    (elif (Variables|Default|GetRedOrWhite)
      (Rendering|Material|SetMaterial (Variables|Default|Getgrapes) 0 "/Game/ImportedAssets/Grape/M_GrapePurple.M_GrapePurple")
      (else
        (Rendering|Material|SetMaterial (Variables|Default|Getgrapes) 0 "/Game/ImportedAssets/Grape/M_GrapeGreen.M_GrapeGreen")))))

(event EventInteract
  (Actor|DestroyActor)
  (bind _asbp_first_person_character (Utilities|Casting|CastToBP_FirstPersonCharacter (Game|GetPlayerCharacter 0)))
  (Default|AddGrapes _asbp_first_person_character)
  (Variables|Default|SetisPicked true)
  (bind _asbp_first_person_character_2 (Utilities|Casting|CastToBP_FirstPersonCharacter (Game|GetPlayerCharacter 0)))
  (bind _result (Math|Integer|IncrementInt (Variables|/Game/FirstPerson/Blueprints/BP_FirstPersonCharacter.BP_FirstPersonCharacter_C|GetNumGrapes _asbp_first_person_character_2))
    (:%20%20
      (Development|PrintString (Utilities|String|ToString(Integer) _result)))))

(fn ConstructionScript)