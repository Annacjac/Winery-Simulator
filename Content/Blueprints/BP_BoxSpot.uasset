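; BP_BoxSpot is an interactable shelf spot where the player can put down a carried box.
; On Interact, it casts the player character to BP_FirstPersonCharacter and, if an item is held and the spot is free, calls PutBoxDown with its Box as the destination.
; It then marks itself occupied and sets itself as the ShelfSpot on the character's CurrentBox.
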(event EventBeginPlay)

(event Collision|EventActorBeginOverlap
  (params (OtherActor :type Actor%20Object%20Reference)))

(event EventTick
  (params (DeltaSeconds :type Float%20%28single-precision%29)))

(event EventInteract
  (bind _asbp_first_person_character (Utilities|Casting|CastToBP_FirstPersonCharacter (Game|GetPlayerCharacter 0)))
  (if (Variables|/Game/FirstPerson/Blueprints/BP_FirstPersonCharacter.BP_FirstPersonCharacter_C|GetHoldingItem _asbp_first_person_character)
    (if (not (Variables|Default|GetisOccupied))
      (Default|PutBoxDown _asbp_first_person_character (Variables|Default|GetBox) (Variables|/Game/FirstPerson/Blueprints/BP_FirstPersonCharacter.BP_FirstPersonCharacter_C|GetCurrentBox _asbp_first_person_character))
      (Variables|Default|SetisOccupied true)
      (Variables|/Game/Blueprints/BP_Box.BP_Box_C|SetShelfSpot (Variables|/Game/FirstPerson/Blueprints/BP_FirstPersonCharacter.BP_FirstPersonCharacter_C|GetCurrentBox _asbp_first_person_character) self))))

(fn ConstructionScript)