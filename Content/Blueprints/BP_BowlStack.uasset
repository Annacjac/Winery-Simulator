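; BP_BowlStack is an interactable bowl dispenser that hands the player wooden bowls and takes empty ones back.
; On Interact, an empty-handed player gets a new BP_WoodBowl, spawned at the character's transform and passed to HoldBowl.
; If the player is already holding an item and CurrentBowl is empty, that bowl is destroyed and HoldingItem is cleared.
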(event EventBeginPlay)

(event Collision|EventActorBeginOverlap
  (params (OtherActor :type Actor%20Object%20Reference)))

(event EventTick
  (params (DeltaSeconds :type Float%20%28single-precision%29)))

(event EventInteract
  (bind _asbp_first_person_character (Utilities|Casting|CastToBP_FirstPersonCharacter (Game|GetPlayerCharacter 0)))
  (if (Variables|/Game/FirstPerson/Blueprints/BP_FirstPersonCharacter.BP_FirstPersonCharacter_C|GetHoldingItem _asbp_first_person_character)
    (if (Variables|/Game/Blueprints/BP_WoodBowl.BP_WoodBowl_C|GetisEmpty (Variables|/Game/FirstPerson/Blueprints/BP_FirstPersonCharacter.BP_FirstPersonCharacter_C|GetCurrentBowl _asbp_first_person_character))
      (Actor|DestroyActor (Variables|/Game/FirstPerson/Blueprints/BP_FirstPersonCharacter.BP_FirstPersonCharacter_C|GetCurrentBowl _asbp_first_person_character))
      (Variables|/Game/FirstPerson/Blueprints/BP_FirstPersonCharacter.BP_FirstPersonCharacter_C|SetHoldingItem _asbp_first_person_character false))
    (else
      (bind _returnvalue (Game|SpawnActorfromClass "/Game/Blueprints/BP_WoodBowl.BP_WoodBowl_C" (Transformation|GetActorTransform _asbp_first_person_character) "Undefined" "MultiplyWithRoot" 0 0))
      (Default|HoldBowl _asbp_first_person_character _returnvalue))))

(fn ConstructionScript)