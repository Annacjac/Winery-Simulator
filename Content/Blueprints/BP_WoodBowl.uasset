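; BP_WoodBowl is an interactable wooden bowl that the player can pick up and that holds either red or white wine.
; Fill and empty events toggle the liquid cylinder's visibility and the IsEmpty flag, while BeginPlay applies the starting state and wine material.
; Interact passes the bowl to the first-person character's HoldBowl and marks its BarrelSpot, if valid, as unoccupied.
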(event Custom|EmptyBowl
  (Rendering|SetVisibility (Variables|Default|GetCylinder) false false)
  (Variables|Default|SetisEmpty true))

(event Custom|FillBowl
  (Rendering|SetVisibility (Variables|Default|GetCylinder) true false)
  (Variables|Default|SetisEmpty false))

(event EventBeginPlay
  (if (Variables|Default|GetisEmpty)
    (CallFunction|EmptyBowl)
    (else
      (CallFunction|FillBowl)
      (if (Variables|Default|GetRedOrWhite)
        (Rendering|Material|SetMaterial (Variables|Default|GetCylinder) 0 "/Game/ImportedAssets/WoodenBowl/M_RedWine.M_RedWine")
        (else
          (Rendering|Material|SetMaterial (Variables|Default|GetCylinder) 0 "/Game/ImportedAssets/WoodenBowl/M_WhiteWine.M_WhiteWine"))))))

(event Collision|EventActorBeginOverlap
  (params (OtherActor :type Actor%20Object%20Reference)))

(event EventTick
  (params (DeltaSeconds :type Float%20%28single-precision%29)))

(event EventInteract
  (bind _barrelspot (Variables|Default|GetBarrelSpot))
  (bind _asbp_first_person_character (Utilities|Casting|CastToBP_FirstPersonCharacter (Game|GetPlayerCharacter 0)))
  (Default|HoldBowl _asbp_first_person_character self)
  (Utilities|IsValid _barrelspot
    (:Is%20Valid
      (Variables|/Game/Blueprints/BP_BowlSpot.BP_BowlSpot_C|SetisOccupied _barrelspot false))))

(fn ConstructionScript)