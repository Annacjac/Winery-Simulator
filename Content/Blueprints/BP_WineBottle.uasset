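; Wine bottle actor that represents a bottle of wine with a price based on how it was made.
; On BeginPlay it splits its comma-separated Description into barrel type, aging time and tannins, and shows the Wine component only if the bottle is full.
; CalculatePrice matches those strings in nested branches, adding to the current Price for aging, then tannins, then barrel, so an unrecognised value skips the later bonuses.
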(event Custom|CalculatePrice
  (bind _barreltype (Variables|Default|GetBarrelType))
  (bind _agingtime (Variables|Default|GetAgingTime))
  (bind _tannins (Variables|Default|GetTannins))
  (if (Utilities|Enum|Equal(Enum) _agingtime "Fermented only")
    (Variables|Default|SetPrice (+ (Variables|Default|GetPrice) 10))
    (if (Utilities|Enum|Equal(Enum) _tannins "tannins removed") :!label _label
      (Variables|Default|SetPrice (+ (Variables|Default|GetPrice) 20))
      (if (Utilities|Enum|Equal(Enum) _barreltype "aged in steel") :!label _label_2
        (Variables|Default|SetPrice (+ (Variables|Default|GetPrice) 10))
        (elif (Utilities|Enum|Equal(Enum) _barreltype "aged in oak")
          (Variables|Default|SetPrice (+ (Variables|Default|GetPrice) 20))))
      (elif (Utilities|Enum|Equal(Enum) _tannins "tannins included")
        (Variables|Default|SetPrice (+ (Variables|Default|GetPrice) 10))
        (goto _label_2)))
    (elif (Utilities|Enum|Equal(Enum) _agingtime "Lightly aged")
      (Variables|Default|SetPrice (+ (Variables|Default|GetPrice) 15))
      (goto _label)
      (elif (Utilities|Enum|Equal(Enum) _agingtime "Heavily aged")
        (Variables|Default|SetPrice (+ (Variables|Default|GetPrice) 20))
        (goto _label)))))

(event EventBeginPlay
  (bind _description (Variables|Default|GetDescription))
  (bind (_lefts _rights) (Utilities|String|Split _description ", "))
  (bind (_lefts_2 _rights_2) (Utilities|String|Split _rights ", "))
  (Variables|Default|SetBarrelType _lefts)
  (Variables|Default|SetAgingTime _lefts_2)
  (Variables|Default|SetTannins _rights_2)
  (if (Variables|Default|GetisFull)
    (Rendering|SetVisibility (Variables|Default|GetWine) true false)
    (else
      (Rendering|SetVisibility (Variables|Default|GetWine) false false))))

(event EventTick
  (params (DeltaSeconds :type Float%20%28single-precision%29)))

(fn ConstructionScript)