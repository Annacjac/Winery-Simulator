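; BP_BowlSpot is an interactable placement spot where the first-person player sets down a carried bowl.
; On Interact, if the player is holding an item and the spot is free, it tells the character to place the current bowl at its Box and marks itself occupied.
; It stores itself on the bowl, then registers that bowl with its parent BP_WoodBarrel, printing a failure message if that cast fails.
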(event Custom|PutDownBowl
  (bind _asbp_first_person_character (Utilities|Casting|CastToBP_FirstPersonCharacter (Game|GetPlayerCharacter 0)))
  (if (Variables|/Game/FirstPerson/Blueprints/BP_FirstPersonCharacter.BP_FirstPersonCharacter_C|GetHoldingItem _asbp_first_person_character)
    (if (not (Variables|Default|GetisOccupied))
      (Default|PutBowlDown _asbp_first_person_character (Variables|Default|GetBox) (Variables|/Game/FirstPerson/Blueprints/BP_FirstPersonCharacter.BP_FirstPersonCharacter_C|GetCurrentBowl _asbp_first_person_character))
      (Variables|Default|SetisOccupied true)
      (bind _output_get (Variables|/Game/Blueprints/BP_WoodBowl.BP_WoodBowl_C|SetBarrelSpot (Variables|/Game/FirstPerson/Blueprints/BP_FirstPersonCharacter.BP_FirstPersonCharacter_C|GetCurrentBowl _asbp_first_person_character) self))
      (bind _asbp_wood_barrel (Utilities|Casting|CastToBP_WoodBarrel (Actor|GetParentActor _output_get))
        (:then
          (Variables|/Game/Blueprints/BP_WoodBarrel.BP_WoodBarrel_C|SetBowl _asbp_wood_barrel (Variables|/Game/FirstPerson/Blueprints/BP_FirstPersonCharacter.BP_FirstPersonCharacter_C|GetCurrentBowl _asbp_first_person_character)))
        (:CastFailed
          (Development|PrintString "failed"))))))

(event EventBeginPlay)

(event Collision|EventActorBeginOverlap
  (params (OtherActor :type Actor%20Object%20Reference)))

(event EventTick
  (params (DeltaSeconds :type Float%20%28single-precision%29)))

(event EventInteract
  (CallFunction|PutDownBowl))

(fn ConstructionScript)