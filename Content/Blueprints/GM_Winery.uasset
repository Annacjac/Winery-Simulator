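; GM_Winery is the Winery game mode, handling player spawn placement and showing the main menu.
; New players restart at the PlayerStart found using the level options string, minus its first character, as the incoming name.
; A MainMenu event creates the UI_MainMenu widget, switches to UI-only input, shows the cursor and ignores movement input.
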(event Custom|MainMenu
  (bind _returnvalue (Game|GetPlayerController 0))
  (bind _returnvalue_2 (UserInterface|CreateWidget "/Game/Blueprints/UI/UI_MainMenu.UI_MainMenu_C"))
  (UserInterface|Viewport|AddtoViewport _returnvalue_2 0)
  (Input|SetInputModeUIOnly _returnvalue _returnvalue_2 "DoNotLock" false)
  (Variables|/Script/Engine.PlayerController|SetbShowMouseCursor _returnvalue true)
  (Input|SetIgnoreMoveInput _returnvalue true))

(event EventBeginPlay)

(event EventTick
  (params (DeltaSeconds :type Float%20%28single-precision%29)))

(event EventHandleStartingNewPlayer
  (params (NewPlayer :type Player%20Controller%20Object%20Reference))
  (bind _optionsstring (Variables|Default|GetOptionsString))
  (Class|GameModeBase|RestartPlayeratPlayerStart NewPlayer (Class|GameModeBase|FindPlayerStart NewPlayer (Utilities|String|GetSubstring _optionsstring 1 (- (Utilities|String|Len _optionsstring) 1)))))

(fn ConstructionScript)