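; BP_StompingBowl is an interactable bowl that the player fills with grapes and stomps until crushed.
; Interact moves grapes from the first-person character's count into the bowl, spawning BP_Grapes at preset spot transforms and recording their variety.
; Once full, stomps advance visual phases at set counts, first destroying every BP_Grapes in the level, later flagging FullyCrushed.
; ClearBowl resets it, and SetCurrentBowl registers it on the character.
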(event Custom|ChangeGrapePhase
  (params (StompCount :type Integer))
  (if (== StompCount 0)
    (Rendering|SetVisibility (Variables|Default|GetGrapesPhase3) false false)
    (Rendering|SetVisibility (Variables|Default|GetPhase2) false false)
    (Variables|Default|SetFullyCrushed false :!label _label)
    (elif (== StompCount 5)
      (Rendering|SetVisibility (Variables|Default|GetPhase2) true false)
      (Rendering|SetVisibility (Variables|Default|GetGrapesPhase3) false false)
      (bind _outactors (Actor|GetAllActorsOfClass "/Game/Blueprints/BP_Grapes.BP_Grapes_C"))
      (for _array_element _outactors
        (Actor|DestroyActor _array_element)
        (goto _label))
      (elif (== StompCount 10)
        (Rendering|SetVisibility (Variables|Default|GetGrapesPhase3) true false)
        (Rendering|SetVisibility (Variables|Default|GetPhase2) false false)
        (Variables|Default|SetFullyCrushed true)))))

(event Custom|SetCurrentBowl
  (bind _asbp_first_person_character (Utilities|Casting|CastToBP_FirstPersonCharacter (Game|GetPlayerCharacter 0)))
  (Variables|/Game/FirstPerson/Blueprints/BP_FirstPersonCharacter.BP_FirstPersonCharacter_C|SetStompingBowl _asbp_first_person_character self))

(event Custom|StompGrape
  (if (Variables|Default|GetIsFull)
    (bind _result (Math|Integer|IncrementInt (Variables|Default|GetStompCount))
      (:%20%20
        (CallFunction|ChangeGrapePhase _result)))))

(event Custom|CreateGrapeArray
  (Variables|Default|SetGrapeSpotsArray (Utilities|Array|MakeArray (Transformation|GetRelativeTransform (Variables|Default|GetBP_GrapeSpot18)) (Transformation|GetRelativeTransform (Variables|Default|GetBP_GrapeSpot4)) (Transformation|GetRelativeTransform (Variables|Default|GetBP_GrapeSpot13)) (Transformation|GetRelativeTransform (Variables|Default|GetBP_GrapeSpot14)) (Transformation|GetRelativeTransform (Variables|Default|GetBP_GrapeSpot15)) (Transformation|GetRelativeTransform (Variables|Default|GetBP_GrapeSpot16)) (Transformation|GetRelativeTransform (Variables|Default|GetBP_GrapeSpot17)) (Transformation|GetRelativeTransform (Variables|Default|GetBP_GrapeSpot11)) (Transformation|GetRelativeTransform (Variables|Default|GetBP_GrapeSpot12)) (Transformation|GetRelativeTransform (Variables|Default|GetBP_GrapeSpot6)) (Transformation|GetRelativeTransform (Variables|Default|GetBP_GrapeSpot7)) (Transformation|GetRelativeTransform (Variables|Default|GetBP_GrapeSpot8)) (Transformation|GetRelativeTransform (Variables|Default|GetBP_GrapeSpot5)) (Transformation|GetRelativeTransform (Variables|Default|GetBP_GrapeSpot9)) (Transformation|GetRelativeTransform (Variables|Default|GetBP_GrapeSpot10)) (Transformation|GetRelativeTransform (Variables|Default|GetBP_GrapeSpot1)) (Transformation|GetRelativeTransform (Variables|Default|GetBP_GrapeSpot19)) (Transformation|GetRelativeTransform (Variables|Default|GetBP_GrapeSpot2)) (Transformation|GetRelativeTransform (Variables|Default|GetBP_GrapeSpot3)) (Transformation|GetRelativeTransform (Variables|Default|GetBP_GrapeSpot4)) (Transformation|GetRelativeTransform (Variables|Default|GetBP_GrapeSpot)))))

(event Custom|AddGrapes
  (bind _grapespotsarray (Variables|Default|GetGrapeSpotsArray))
  (bind _grapespotindex (Variables|Default|GetGrapeSpotIndex))
  (bind _output (Utilities|Array|Get(acopy) _grapespotsarray _grapespotindex))
  (if (not (Variables|Default|GetIsFull))
    (bind _returnvalue (Game|SpawnActorfromClass "/Game/Blueprints/BP_Grapes.BP_Grapes_C" (Variables|Default|GetOrigin) "Undefined" "MultiplyWithRoot" 0 0))
    (Variables|Default|Setvariety (Variables|/Game/Blueprints/BP_Grapes.BP_Grapes_C|GetVariety _returnvalue))
    (Collision|SetActorEnableCollision _returnvalue false)
    (Math|Integer|IncrementInt _grapespotindex
      (:%20%20
        (Transformation|SetWorldLocationAndRotation (Variables|/Script/Engine.Actor|GetRootComponent _returnvalue) (+ (Transformation|GetActorLocation) (Math|Transform|TransformLocation _output "0, 0, 0")) (Math|Transform|TransformRotation _output "0, 0, 0") false false)
        (Transformation|SetWorldScale3D (Variables|/Script/Engine.Actor|GetRootComponent _returnvalue) "0.035000,0.035000,0.035000")
        (if (== _grapespotindex (- (Utilities|Array|Length _grapespotsarray) 1))
          (Variables|Default|SetIsFull true))))))

(event Custom|ClearBowl
  (if (Variables|Default|GetIsFull)
    (Variables|Default|SetStompCount 0)
    (CallFunction|ChangeGrapePhase)
    (Variables|Default|SetIsFull false)
    (Variables|Default|SetGrapeSpotIndex 0)
    (Variables|Default|SetnumGrapes 0)
    (Variables|Default|SetFullyCrushed false)))

(event EventBeginPlay
  (CallFunction|CreateGrapeArray)
  (CallFunction|ChangeGrapePhase))

(event Collision|EventActorBeginOverlap
  (params (OtherActor :type Actor%20Object%20Reference)))

(event EventTick
  (params (DeltaSeconds :type Float%20%28single-precision%29)))

(event EventInteract
  (bind _numgrapes (Variables|Default|GetnumGrapes))
  (bind _asbp_first_person_character (Utilities|Casting|CastToBP_FirstPersonCharacter (Game|GetPlayerCharacter 0)))
  (if (== (Variables|Default|GetnumGrapes) 20)
    (Variables|Default|SetIsFull true)
    (elif (and (< _numgrapes 20) (> (Variables|/Game/FirstPerson/Blueprints/BP_FirstPersonCharacter.BP_FirstPersonCharacter_C|GetNumGrapes _asbp_first_person_character) 0))
      (CallFunction|AddGrapes)
      (Math|Integer|DecrementInt (Variables|/Game/FirstPerson/Blueprints/BP_FirstPersonCharacter.BP_FirstPersonCharacter_C|GetNumGrapes _asbp_first_person_character)
        (:%20%20
          (Math|Integer|IncrementInt _numgrapes))))))

(fn ConstructionScript)