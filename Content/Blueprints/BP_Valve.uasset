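; BP_Valve is an interactable valve, parented to a BP_StompingBowl, that sends crushed grapes on to barrels for aging.
; Interacting toggles its rotation and, if the bowl is fully crushed, opens UI_AgingOptions with mouse-only UI input.
; Tick polls a Confirmed flag, then transfers grapes and clears the bowl.
; Wood transfers begin aging in the first non-full BP_WoodBarrel; the Steel branch loops over barrels without acting.
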(event Custom|TurnValve
  (if (Variables|Default|GetPosition)
    (Transformation|SetActorRotation (Math|Conversions|RotationFromXVector (Math|Vector|RotateVector "0.000000,90.000000,0.000000" (Transformation|GetActorRotation))))
    (Variables|Default|SetPosition false)
    (else
      (Transformation|SetActorRotation (Math|Conversions|RotationFromXVector (Math|Vector|RotateVector "0.000000,-90.000000,0.000000" (Transformation|GetActorRotation))))
      (Variables|Default|SetPosition true))))

(event Custom|TransferGrapes
  (if (Utilities|Enum|Equal(Enum) (Variables|Default|GetbarrelType) "Wood")
    (bind _outactors (Actor|GetAllActorsOfClass "/Game/Blueprints/BP_WoodBarrel.BP_WoodBarrel_C"))
    (bind _array_element (Utilities|Array|ForEachLoopwithBreak _outactors :!label _label)
      (:LoopBody
        (if (not (Variables|/Game/Blueprints/BP_WoodBarrel.BP_WoodBarrel_C|GetisFull _array_element))
          (Default|BeginAging _array_element (Variables|/Game/Blueprints/BP_StompingBowl.BP_StompingBowl_C|Getvariety (Variables|Default|GetBowl)) (Variables|Default|GetdesiredAgeTime) (Variables|Default|GetTanninRemoved))
          (goto _label Break))))
    (elif (Utilities|Enum|Equal(Enum) (Variables|Default|GetbarrelType) "Steel")
      (bind _outactors_2 (Actor|GetAllActorsOfClass "/Game/Blueprints/BP_SteelBarrel.BP_SteelBarrel_C"))
      (Utilities|Array|ForEachLoopwithBreak _outactors_2))))

(event EventBeginPlay)

(event Collision|EventActorBeginOverlap
  (params (OtherActor :type Actor%20Object%20Reference)))

(event EventTick
  (params (DeltaSeconds :type Float%20%28single-precision%29))
  (bind _returnvalue (Actor|GetParentActor))
  (if (Variables|Default|GetConfirmed)
    (CallFunction|TransferGrapes)
    (Utilities|IsValid _returnvalue
      (:Is%20Valid
        (bind _asbp_stomping_bowl (Utilities|Casting|CastToBP_StompingBowl _returnvalue))
        (Default|ClearBowl _asbp_stomping_bowl)
        (Variables|Default|SetConfirmed false)))))

(event EventInteract
  (bind _returnvalue (Actor|GetParentActor))
  (bind _returnvalue_2 (Game|GetPlayerController 0))
  (CallFunction|TurnValve)
  (Utilities|IsValid _returnvalue
    (:Is%20Valid
      (bind _asbp_stomping_bowl (Utilities|Casting|CastToBP_StompingBowl _returnvalue))
      (bind _output_get (Variables|Default|SetBowl _asbp_stomping_bowl))
      (if (Variables|/Game/Blueprints/BP_StompingBowl.BP_StompingBowl_C|GetFullyCrushed _output_get)
        (bind _returnvalue_3 (UserInterface|CreateWidget "/Game/Blueprints/UI/UI_AgingOptions.UI_AgingOptions_C"))
        (Variables|/Game/Blueprints/UI/UI_AgingOptions.UI_AgingOptions_C|SetValve _returnvalue_3 self)
        (UserInterface|Viewport|AddtoViewport _returnvalue_3 0)
        (Input|SetInputModeUIOnly _returnvalue_2 0 "DoNotLock" false)
        (Variables|/Script/Engine.PlayerController|SetbShowMouseCursor _returnvalue_2 true)))))

(fn ConstructionScript)