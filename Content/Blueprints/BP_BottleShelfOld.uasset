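; Wine bottle shelf actor that stocks itself on BeginPlay and serves as an interactable bottle inventory.
; FillShelf spawns a BP_WineBottle at each of its box components, which act as placement slots, aligning it to the shelf with collision off and storing it in BottleArray.
; Interact adds the player's held bottle to the array under a Quantity cap, or otherwise registers the shelf on the character and opens UI_BottleInventory with mouse input.
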(event Custom|FillShelf
  (for _array_element (Actor|GetComponentsByClass "/Script/Engine.BoxComponent")
    (bind _returnvalue (Game|SpawnActorfromClass "/Game/Blueprints/BP_WineBottle.BP_WineBottle_C" (Variables|Default|GetOrigin) "Undefined" "MultiplyWithRoot" 0 0))
    (bind _returnvalue_2 (Utilities|Array|Add (Variables|Default|GetBottleArray) _returnvalue))
    (Variables|Default|SetQuantity _returnvalue_2)
    (Transformation|SetWorldLocation (Variables|/Script/Engine.Actor|GetRootComponent _returnvalue) (Transformation|GetWorldLocation _array_element) false false)
    (Transformation|SetRelativeRotation (Variables|/Script/Engine.Actor|GetRootComponent _returnvalue) (Transformation|GetWorldRotation (Variables|Transformation|GetRootComponent self)) false false)
    (Transformation|AddRelativeRotation (Variables|/Script/Engine.Actor|GetRootComponent _returnvalue) "90.000000,0.000000,0.000000" false false)
    (Collision|SetActorEnableCollision _returnvalue false)))

(event EventBeginPlay
  (CallFunction|FillShelf))

(event Collision|EventActorBeginOverlap
  (params (OtherActor :type Actor%20Object%20Reference)))

(event EventTick
  (params (DeltaSeconds :type Float%20%28single-precision%29)))

(event EventInteract
  (bind _returnvalue (Game|GetPlayerController 0))
  (bind _asbp_first_person_character (Utilities|Casting|CastToBP_FirstPersonCharacter (Game|GetPlayerCharacter 0)))
  (if (and (Variables|/Game/FirstPerson/Blueprints/BP_FirstPersonCharacter.BP_FirstPersonCharacter_C|GetHoldingItem _asbp_first_person_character) (Utilities|Enum|Equal(Enum) (Variables|/Game/FirstPerson/Blueprints/BP_FirstPersonCharacter.BP_FirstPersonCharacter_C|GetitemHeld _asbp_first_person_character) "bottle"))
    (if (< (Variables|Default|GetQuantity) 122)
      (bind _asbp_first_person_character_2 (Utilities|Casting|CastToBP_FirstPersonCharacter (Game|GetPlayerCharacter 0)))
      (Utilities|Array|Add (Variables|Default|GetBottleArray) (Variables|/Game/FirstPerson/Blueprints/BP_FirstPersonCharacter.BP_FirstPersonCharacter_C|GetCurrentBottle _asbp_first_person_character_2)))
    (else
      (Variables|/Game/FirstPerson/Blueprints/BP_FirstPersonCharacter.BP_FirstPersonCharacter_C|SetShelf _asbp_first_person_character self)
      (Input|SetInputModeUIOnly _returnvalue 0 "DoNotLock" false)
      (bind _returnvalue_2 (UserInterface|CreateWidget "/Game/Blueprints/UI/UI_BottleInventory.UI_BottleInventory_C"))
      (UserInterface|Viewport|AddtoViewport _returnvalue_2 0)
      (Variables|/Script/Engine.PlayerController|SetbShowMouseCursor _returnvalue true))))

(fn ConstructionScript)