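; BP_Pallet is an interactable pallet where the first-person player sets down carried boxes, up to 18 in total.
; On BeginPlay it caches the relative transforms of its 18 Box components as slot positions.
; Interact detaches the held box, teleports it to a location computed from the next slot transform and the pallet's location, advances the index, clears HoldingItem and calls CloseBox.
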(event Custom|CreateSpotsArray
  (Variables|Default|SetBoxTransformArray (Utilities|Array|MakeArray (Transformation|GetRelativeTransform (Variables|Default|GetBox)) (Transformation|GetRelativeTransform (Variables|Default|GetBox1)) (Transformation|GetRelativeTransform (Variables|Default|GetBox2)) (Transformation|GetRelativeTransform (Variables|Default|GetBox3)) (Transformation|GetRelativeTransform (Variables|Default|GetBox4)) (Transformation|GetRelativeTransform (Variables|Default|GetBox5)) (Transformation|GetRelativeTransform (Variables|Default|GetBox6)) (Transformation|GetRelativeTransform (Variables|Default|GetBox7)) (Transformation|GetRelativeTransform (Variables|Default|GetBox8)) (Transformation|GetRelativeTransform (Variables|Default|GetBox9)) (Transformation|GetRelativeTransform (Variables|Default|GetBox10)) (Transformation|GetRelativeTransform (Variables|Default|GetBox11)) (Transformation|GetRelativeTransform (Variables|Default|GetBox12)) (Transformation|GetRelativeTransform (Variables|Default|GetBox13)) (Transformation|GetRelativeTransform (Variables|Default|GetBox14)) (Transformation|GetRelativeTransform (Variables|Default|GetBox15)) (Transformation|GetRelativeTransform (Variables|Default|GetBox16)) (Transformation|GetRelativeTransform (Variables|Default|GetBox17)))))

(event Custom|Pallet%20Add%20Box
  (params (Box :type BP%20Box%20Object%20Reference) (Index :type Integer))
  (Transformation|SetWorldTransform (Variables|/Script/Engine.Actor|GetRootComponent Box) (Math|Conversions|ToTransform(Vector) (Math|Transform|TransformLocation (Utilities|Array|Get(acopy) (Variables|Default|GetBoxTransformArray) Index) (Transformation|GetActorLocation))) false true))

(event EventBeginPlay
  (CallFunction|CreateSpotsArray)
  (Variables|Default|SetCurrentIndex 0))

(event Collision|EventActorBeginOverlap
  (params (OtherActor :type Actor%20Object%20Reference)))

(event EventTick
  (params (DeltaSeconds :type Float%20%28single-precision%29)))

(event EventInteract
  (if (< (Variables|Default|GetCurrentIndex) 18)
    (bind _asbp_first_person_character (Utilities|Casting|CastToBP_FirstPersonCharacter (Game|GetPlayerCharacter 0)))
    (if (Variables|/Game/FirstPerson/Blueprints/BP_FirstPersonCharacter.BP_FirstPersonCharacter_C|GetHoldingItem _asbp_first_person_character)
      (bind _currentbox (Default|GetCurrentBox _asbp_first_person_character))
      (Transformation|DetachFromActor _currentbox "KeepRelative" "KeepRelative" "KeepRelative")
      (CallFunction|PalletAddBox _currentbox (Variables|Default|GetCurrentIndex))
      (bind _result (Math|Integer|IncrementInt (Variables|Default|GetCurrentIndex))
        (:%20%20
          (Variables|Default|SetCurrentIndex _result)
          (Variables|/Game/FirstPerson/Blueprints/BP_FirstPersonCharacter.BP_FirstPersonCharacter_C|SetHoldingItem _asbp_first_person_character false)
          (Default|CloseBox _currentbox))))))

(fn ConstructionScript)