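; BP_Box is an interactable box that the player can pick up and hold, with open and closed states.
; OpenBox and CloseBox set IsOpen and toggle visibility between two static meshes, and BeginPlay applies the initial state.
; Interact opens the box, passes it to BP_FirstPersonCharacter's HoldBox and marks any valid ShelfSpot as unoccupied.
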(event Custom|OpenBox
  (Variables|Default|SetisOpen true)
  (Rendering|SetVisibility (Variables|Default|GetSM_BoxClosed) false false)
  (Rendering|SetVisibility (Variables|Default|GetSM_BoxOpen) true false))

(event Custom|CloseBox
  (Variables|Default|SetisOpen false)
  (Rendering|SetVisibility (Variables|Default|GetSM_BoxOpen) false false)
  (Rendering|SetVisibility (Variables|Default|GetSM_BoxClosed) true false))

(event EventBeginPlay
  (if (Variables|Default|GetisOpen)
    (Rendering|SetVisibility (Variables|Default|GetSM_BoxClosed) false false)
    (Rendering|SetVisibility (Variables|Default|GetSM_BoxOpen) true false)
    (else
      (Rendering|SetVisibility (Variables|Default|GetSM_BoxOpen) false false)
      (Rendering|SetVisibility (Variables|Default|GetSM_BoxClosed) true false))))

(event EventInteract
  (bind _shelfspot (Variables|Default|GetShelfSpot))
  (bind _asbp_first_person_character (Utilities|Casting|CastToBP_FirstPersonCharacter (Game|GetPlayerCharacter 0)))
  (CallFunction|OpenBox)
  (bind _output_get (Variables|Default|SetCurrentBox self))
  (Default|HoldBox _asbp_first_person_character _output_get)
  (Utilities|IsValid _shelfspot
    (:Is%20Valid
      (Variables|/Game/Blueprints/BP_BoxSpot.BP_BoxSpot_C|SetisOccupied _shelfspot false))))

(fn ConstructionScript)